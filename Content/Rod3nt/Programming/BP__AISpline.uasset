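; BP__AISpline is a patrol path actor that supplies AI with successive world locations along a spline.
; IncrementPath advances a point index by the current direction, reversing at the last or first spline point so the route ping-pongs.
; SplinePath returns the world-space location of the current point.
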(event `Increment Path`
  (bind _output_get (set `self.Path Point` (+ (`self.Path Point`) (`self.Direction`))))
  (if (== _output_get (- (`SplineComponent.GetNumberOfSplinePoints` (`self.Spline`)) 1))
    (set `self.Direction` -1)
    (elif (== (`self.Path Point`) 0)
      (set `self.Direction` 1))))

(fn `Spline Path`
  (returns (LOC :type "Vector Structure"))
  (return (`SplineComponent.GetLocationAtSplinePoint` (`self.Spline`) (`self.Path Point`) "World")))

(fn `UserConstructionScript`)